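; BP_LightSwitch is an interactable light switch that lets the player toggle a referenced light while standing near it.
; BeginPlay hides the prompt text and the light and disables input.
; Box overlap enables player input and shows the TextRender prompt, while end overlap disables input and hides it again.
; The Interact action flips the LightOff flag and toggles the visibility of MyLight's light component.
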(event OnComponentBeginOverlap(Box)
  (params (OverlappedComponent :type Primitive%20Component%20Object%20Reference) (OtherActor :type Actor%20Object%20Reference) (OtherComp :type Primitive%20Component%20Object%20Reference) (OtherBodyIndex :type Integer) (bFromSweep :type Boolean) (SweepResult :type Hit%20Result%20Structure%20%28by%20ref%29))
  ;[1 1 1] Comment
  (Variables|Default|SetInBox true)
  (Input|EnableInput (Game|GetPlayerController 0))
  (Rendering|SetVisibility (Variables|Default|GetTextRender) (Variables|Default|GetInBox) false))

(event OnComponentEndOverlap(Box)
  (params (OverlappedComponent :type Primitive%20Component%20Object%20Reference) (OtherActor :type Actor%20Object%20Reference) (OtherComp :type Primitive%20Component%20Object%20Reference) (OtherBodyIndex :type Integer))
  ;[1 1 1] Comment
  (Variables|Default|SetInBox false)
  (Input|DisableInput (Game|GetPlayerController 0))
  (Rendering|SetVisibility (Variables|Default|GetTextRender) (Variables|Default|GetInBox) false))

(event EventBeginPlay
  (Rendering|SetVisibility (Variables|Default|GetTextRender) false false)
  (Rendering|SetVisibility (Variables|/Script/Engine.Light|GetLightComponent (Variables|Default|GetMyLight)) false false)
  (Input|DisableInput (Game|GetPlayerController 0)))

(event Input|ActionEvents|InputActionInteract
  (params (Key :type Key%20Structure :default "None"))
  ;[1 1 1] Comment
  (:Pressed
    (Variables|Default|SetlightOff (not (Variables|Default|GetlightOff)))
    (Rendering|ToggleVisibility (Variables|/Script/Engine.Light|GetLightComponent (Variables|Default|GetMyLight)) false)))

(fn ConstructionScript)